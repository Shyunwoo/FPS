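; BP_Khaimera is the Khaimera enemy Blueprint, adding health bar and floating damage number UI on top of its parent class.
; On BeginPlay it links itself to the WBP_EnemyHealthBar widget and hides it until the show event fires.
; ShowHitNumber spawns a WBP_HitNumber at the hit's projected screen position, registers it through StoreHitNumber, then sets damage and headshot data and plays its animation.
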(event `self.ReceiveBeginPlay`
  (`parent.ReceiveBeginPlay`)
  (bind _aswbp_enemy_health_bar (cast `/Game/_Game/_Blueprints/HUD/WBP_EnemyHealthBar` (`WidgetComponent.GetUserWidgetObject` (`self.HealthBar`))))
  (set `/Game/_Game/_Blueprints/HUD/WBP_EnemyHealthBar.Enemy` self _aswbp_enemy_health_bar)
  (`Widget.SetVisibility` (`WidgetComponent.GetUserWidgetObject` (`self.HealthBar`)) "Hidden"))

(event `self.ShowHealthBar`
  (bind _returnvalue (`WidgetComponent.GetUserWidgetObject` (`self.HealthBar`)))
  (`/Engine/EditorBlueprintResources/StandardMacros.IsValid` _returnvalue
    (:`Is Valid`
      (`Widget.SetVisibility` _returnvalue "Visible")
      (`parent.ShowHealthBar`))))

(event `self.HideHealthBar`
  (bind _returnvalue (`WidgetComponent.GetUserWidgetObject` (`self.HealthBar`)))
  (`/Engine/EditorBlueprintResources/StandardMacros.IsValid` _returnvalue
    (:`Is Valid`
      (`Widget.SetVisibility` _returnvalue "Hidden"))))

(event `self.ShowHitNumber`
  (params (Damage :type Integer) (HitLocation :type "Vector Structure") (bHeadShot :type Boolean))
  (bind _returnvalue (`|CreateWidget` "/Game/_Game/_Blueprints/HUD/WBP_HitNumber.WBP_HitNumber_C"))
  (`UserWidget.AddToViewport` _returnvalue 0)
  (`UserWidget.SetPositionInViewport` _returnvalue (`GameplayStatics.ProjectWorldToScreen` (`GameplayStatics.GetPlayerController` 0) HitLocation) true)
  (`self.StoreHitNumber` _returnvalue HitLocation)
  (set `/Game/_Game/_Blueprints/HUD/WBP_HitNumber.HitText` (`KismetTextLibrary.Conv_IntToText` Damage) _returnvalue)
  (set `/Game/_Game/_Blueprints/HUD/WBP_HitNumber.HeadShot` bHeadShot _returnvalue)
  (`UserWidget.PlayAnimation` _returnvalue (`/Game/_Game/_Blueprints/HUD/WBP_HitNumber.HitNumberAnimation` _returnvalue) 0.0 1 "Forward" 1.0 false))

(fn `UserConstructionScript`)