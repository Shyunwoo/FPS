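; BP_FPSHUD is the first-person HUD that draws a dynamic crosshair from the equipped weapon's textures.
; It caches the player's BP_FPSCharacter on BeginPlay and re-fetches it during DrawHUD if the reference is invalid.
; Each frame it draws five pieces around screen center, pushing the top, bottom, left and right ones outward by the character's spread multiplier times a maximum spread.
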(event `self.ReceiveBeginPlay`
  (`/Engine/EditorBlueprintResources/StandardMacros.IsValid` (`self.FPSCharacter`)
    (:`Is Not Valid`
      (bind _asbp_fpscharacter (cast `/Game/_Game/_Blueprints/_Character/BP_FPSCharacter` (`GameplayStatics.GetPlayerPawn` 0)))
      (set `self.FPSCharacter` _asbp_fpscharacter))))

(event `self.ReceiveDrawHUD`
  (params (SizeX :type Integer) (SizeY :type Integer))
  (bind (_x _y) (`KismetMathLibrary.BreakVector2D` (`self.CrosshairbaseCenter`)))
  (bind (_x_2 _y_2) (`KismetMathLibrary.BreakVector2D` (`self.CrosshairbaseCenter`)))
  (bind (_x_3 _y_3) (`KismetMathLibrary.BreakVector2D` (`self.CrosshairbaseCenter`)))
  (bind (_x_4 _y_4) (`KismetMathLibrary.BreakVector2D` (`self.CrosshairbaseCenter`)))
  (bind (_x_5 _y_5) (`KismetMathLibrary.BreakVector2D` (`self.CrosshairbaseCenter`)))
  (bind (_x_6 _y_6) (`KismetMathLibrary.BreakVector2D` (`self.CrosshairLocation`)))
  (set `self.ScreenCenter` (`KismetMathLibrary.MakeVector2D` (`KismetMathLibrary.Conv_IntToDouble` (/ SizeX 2)) (`KismetMathLibrary.Conv_IntToDouble` (/ SizeY 2))))
  (set `self.CrosshairLocation` (`self.ScreenCenter`))
  (`/Engine/EditorBlueprintResources/StandardMacros.IsValid` (`self.FPSCharacter`)
    (:`Is Valid`
      _)
    (:`Is Not Valid`
      (bind _asbp_fpscharacter (cast `/Game/_Game/_Blueprints/_Character/BP_FPSCharacter` (`GameplayStatics.GetPlayerPawn` 0)))
      (set `self.FPSCharacter` _asbp_fpscharacter)))
  (set `self.CrosshairSpreadMultiplier` (`FPSCharacter.GetCrosshairSpreadMultiplier` (`self.FPSCharacter`)))
  (set `self.CrosshairbaseCenter` (`KismetMathLibrary.MakeVector2D` (- _x_6 (`self.CrosshairHalfWidth`)) (- _y_6 (`self.CrosshairHalfHeight`))))
  (`|ExecutionSequence`
    (:`then_0`
      (`self.DrawTexture` (`Weapon.CrosshairsBottom` (`FPSCharacter.EquippedWeapon` (`self.FPSCharacter`))) _x_3 (+ _y_3 (* (`self.CrosshairSpreadMultiplier`) (`self.CrosshairSpeadMax`))) 64.0 64.0 0.0 0.0 1.0 1.0))
    (:`then_1`
      (`self.DrawTexture` (`Weapon.CrosshairsTop` (`FPSCharacter.EquippedWeapon` (`self.FPSCharacter`))) _x_4 (- _y_4 (* (`self.CrosshairSpreadMultiplier`) (`self.CrosshairSpeadMax`))) 64.0 64.0 0.0 0.0 1.0 1.0))
    (:`then_2`
      (`self.DrawTexture` (`Weapon.CrosshairsLeft` (`FPSCharacter.EquippedWeapon` (`self.FPSCharacter`))) (- _x_5 (* (`self.CrosshairSpreadMultiplier`) (`self.CrosshairSpeadMax`))) _y_5 64.0 64.0 0.0 0.0 1.0 1.0))
    (:`then_3`
      (`self.DrawTexture` (`Weapon.CrosshairsRight` (`FPSCharacter.EquippedWeapon` (`self.FPSCharacter`))) (+ _x (* (`self.CrosshairSpreadMultiplier`) (`self.CrosshairSpeadMax`))) _y 64.0 64.0 0.0 0.0 1.0 1.0))
    (:`then_4`
      (`self.DrawTexture` (`Weapon.CrosshairsMiddle` (`FPSCharacter.EquippedWeapon` (`self.FPSCharacter`))) _x_2 _y_2 64.0 64.0 0.0 0.0 1.0 1.0))))

(fn `UserConstructionScript`)